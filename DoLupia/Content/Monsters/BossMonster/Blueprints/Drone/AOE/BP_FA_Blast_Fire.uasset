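; BP_FA_Blast_Fire is a blast effect actor, filed under the boss monster's drone AOE Blueprints, that grows into view when spawned.
; BeginPlay sets its scale to zero and spawns the NS_Lightning_strike effect at its location.
; Tick eases its rotation toward a fixed 180-degree turn with a per-frame lerp and grows its scale by delta time until about full size.
; The graphs contain no damage or destroy logic.
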(event EventBeginPlay
  (Transformation|SetActorScale3D "0, 0, 0")
  (Niagara|SpawnSystematLocation "/Game/WizardSpellsPack/Effects/NS_Lightning_strike.NS_Lightning_strike" (Transformation|GetActorLocation)))

(event EventTick
  (params (DeltaSeconds :type Float%20%28single-precision%29))
  (Transformation|SetActorRotation (Math|Rotator|Lerp(Rotator) (Transformation|GetActorRotation) "0.000000,180.000000,0.000000" 0.125 true))
  (if (<= (.x (Transformation|GetActorScale3D)) 1.0)
    (Transformation|SetActorScale3D (+ (* (Utilities|Time|GetWorldDeltaSeconds) 2.0) (Transformation|GetActorScale3D)))))

(fn ConstructionScript)
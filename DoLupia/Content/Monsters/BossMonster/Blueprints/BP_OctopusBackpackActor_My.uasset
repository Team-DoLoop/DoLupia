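; Octopus backpack actor for the boss monster, adding finger-curl IK and trail effects to its tentacle hands.
; Tick box-traces between hand sockets on attached or grabbing hands, raising two-stage section curl values until contact; attach and grab events reset them.
; Tick also sets GrabTarget from hand states, hides the player pawn on a grab and turns an arrow toward the camera.
; Attack and move events attach Niagara trails; return destroys stored ones.
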(event EventTick
  (params (DeltaSeconds :type Float%20%28single-precision%29))
  (bind _arrow (Variables|Default|GetArrow))
  ;[1 0.5563 0] For Animation Hand IK
  (for _array_element (Variables|Default|GettentaclesArr)
    (if (Math|Boolean|ORBoolean (Utilities|Enum|Equal(Enum) (.action (Utilities|Struct|BreakOctoHandStatus (Utilities|Array|Get(acopy) (Variables|/Script/OctopusBackpack.OctopusBackpackComponent|GethandsArr (.backpackComponent (Utilities|Struct|BreakOctoTentaclesStruct _array_element)))))) "GRABBED") (Utilities|Enum|Equal(Enum) (.action (Utilities|Struct|BreakOctoHandStatus (Utilities|Array|Get(acopy) (Variables|/Script/OctopusBackpack.OctopusBackpackComponent|GethandsArr (.backpackComponent (Utilities|Struct|BreakOctoTentaclesStruct _array_element))) 1))) "GRABBED") (Utilities|Enum|Equal(Enum) (.action (Utilities|Struct|BreakOctoHandStatus (Utilities|Array|Get(acopy) (Variables|/Script/OctopusBackpack.OctopusBackpackComponent|GethandsArr (.backpackComponent (Utilities|Struct|BreakOctoTentaclesStruct _array_element))) 2))) "GRABBED") (Utilities|Enum|Equal(Enum) (.action (Utilities|Struct|BreakOctoHandStatus (Utilities|Array|Get(acopy) (Variables|/Script/OctopusBackpack.OctopusBackpackComponent|GethandsArr (.backpackComponent (Utilities|Struct|BreakOctoTentaclesStruct _array_element))) 3))) "GRABBED"))
      (Development|PrintString "Grabbed")
      (Variables|Default|SetGrabTarget true)
      (Rendering|SetActorHiddenInGame (Game|Player|GetPlayerPawn 0) true)
      (else
        (Development|PrintString "Not Grabbed" true true "(R=1.000000,G=0.473421,B=0.000000,A=1.000000)")
        (Variables|Default|SetGrabTarget false))))
  (for (_array_element_2 _array_index) (Variables|Default|GettentaclesArr)
    (Utilities|IsValid (.backpackComponent (Utilities|Struct|BreakOctoTentaclesStruct _array_element_2))
      (:Is%20Valid
        (Utilities|IsValid (.handSkeletalComponent (Utilities|Struct|BreakOctoTentaclesStruct _array_element_2))
          (:Is%20Valid
            (if (or (Utilities|Enum|Equal(Enum) (.action (Utilities|Struct|BreakOctoHandStatus (Utilities|Array|Get(acopy) (Variables|/Script/OctopusBackpack.OctopusBackpackComponent|GethandsArr (.backpackComponent (Utilities|Struct|BreakOctoTentaclesStruct _array_element_2))) _array_index))) "ATTACHED") (Utilities|Enum|Equal(Enum) (.action (Utilities|Struct|BreakOctoHandStatus (Utilities|Array|Get(acopy) (Variables|/Script/OctopusBackpack.OctopusBackpackComponent|GethandsArr (.backpackComponent (Utilities|Struct|BreakOctoTentaclesStruct _array_element_2))) _array_index))) "GRABBED"))
              (bind _output_get (Variables|Default|SetHandSkeletalComponent (.handSkeletalComponent (Utilities|Struct|BreakOctoTentaclesStruct _array_element_2))))
              (Variables|Default|SetMeshRotation (Transformation|GetWorldRotation _output_get))
              (bind _output_get_2 (Variables|Default|SetHandIndex (.handIndex (Utilities|Struct|BreakOctoTentaclesStruct _array_element_2))))
              (for (_ _array_index_2) (.SocketFirstStartArr (Utilities|Struct|BreakS_OctoHandAnim (Utilities|Array|Get(acopy) (Variables|Default|GetOctoHandAnimStruct) _output_get_2)))
                (Variables|Default|SetSectionIndex _array_index_2)
                (bind _returnvalue (Collision|BoxTraceByChannel (Transformation|GetSocketLocation (Variables|Default|GetHandSkeletalComponent) (Utilities|Array|Get(acopy) (.SocketFirstStartArr (Utilities|Struct|BreakS_OctoHandAnim (Utilities|Array|Get(acopy) (Variables|Default|GetOctoHandAnimStruct) _output_get_2))) (Variables|Default|GetSectionIndex))) (Transformation|GetSocketLocation (Variables|Default|GetHandSkeletalComponent) (Utilities|Array|Get(acopy) (.SocketFirstEndArr (Utilities|Struct|BreakS_OctoHandAnim (Utilities|Array|Get(acopy) (Variables|Default|GetOctoHandAnimStruct) _output_get_2))) (Variables|Default|GetSectionIndex))) "3.000000,5.000000,1.000000" (Variables|Default|GetMeshRotation) "TraceTypeQuery1" false 0 "None"))
                (bind _returnvalue_2 (Collision|BoxTraceByChannel (Transformation|GetSocketLocation (Variables|Default|GetHandSkeletalComponent) (Utilities|Array|Get(acopy) (.SocketSecondStartArr (Utilities|Struct|BreakS_OctoHandAnim (Utilities|Array|Get(acopy) (Variables|Default|GetOctoHandAnimStruct) (Variables|Default|GetHandIndex)))) (Variables|Default|GetSectionIndex))) (Transformation|GetSocketLocation (Variables|Default|GetHandSkeletalComponent) (Utilities|Array|Get(acopy) (.SocketSecondEndArr (Utilities|Struct|BreakS_OctoHandAnim (Utilities|Array|Get(acopy) (Variables|Default|GetOctoHandAnimStruct) (Variables|Default|GetHandIndex)))) (Variables|Default|GetSectionIndex))) "3.000000,5.000000,1.000000" (Variables|Default|GetMeshRotation) "TraceTypeQuery1" false 0 "None"))
                (if (and (not _returnvalue_2) (not _returnvalue))
                  (Utilities|Array|SetArrayElem (.FirstSection (Utilities|Struct|BreakS_OctoHandAnim (Utilities|Array|Get(acopy) (Variables|Default|GetOctoHandAnimStruct) (Variables|Default|GetHandIndex)))) (Variables|Default|GetSectionIndex) (+ (Utilities|Array|Get(acopy) (.FirstSection (Utilities|Struct|BreakS_OctoHandAnim (Utilities|Array|Get(acopy) (Variables|Default|GetOctoHandAnimStruct) (Variables|Default|GetHandIndex)))) (Variables|Default|GetSectionIndex)) (* (Utilities|Time|GetWorldDeltaSeconds) 25.0)))
                  (Utilities|Array|SetArrayElem (.SecondSection (Utilities|Struct|BreakS_OctoHandAnim (Utilities|Array|Get(acopy) (Variables|Default|GetOctoHandAnimStruct) (Variables|Default|GetHandIndex)))) (Variables|Default|GetSectionIndex) (+ (Utilities|Array|Get(acopy) (.SecondSection (Utilities|Struct|BreakS_OctoHandAnim (Utilities|Array|Get(acopy) (Variables|Default|GetOctoHandAnimStruct) (Variables|Default|GetHandIndex)))) (Variables|Default|GetSectionIndex)) (* (Utilities|Time|GetWorldDeltaSeconds) 25.0)) :!label _label)
                  (elif (not _returnvalue_2)
                    (goto _label))))))))))
  ;[0.2257 0.7778 1] Auto Rotate Widget
  (Transformation|SetWorldRotation _arrow (Math|Rotator|FindLookatRotation (Transformation|GetWorldLocation _arrow) (Camera|GetCameraLocation (Game|GetPlayerCameraManager 0))) false false))

(event EventReturnEvent
  (params (tentacle :type Octo%20Tentacles%20Struct%20Structure))
  ;[1 1 1] Reset Trail Effect
  (for _array_element (Variables|Default|GetNS_TrailsArr)
    (if (Utilities|Enum|Equal(Enum) (.Hand (Utilities|Struct|BreakS_OctoHand _array_element)) (.hand (Utilities|Struct|BreakOctoTentaclesStruct tentacle)))
      (Utilities|IsValid (.NS_Trail (Utilities|Struct|BreakS_OctoHand _array_element))
        (:Is%20Valid
          (Components|DestroyComponent (.NS_Trail (Utilities|Struct|BreakS_OctoHand _array_element))))))))

(event EventAttackMoveEvent
  (params (tentacle :type Octo%20Tentacles%20Struct%20Structure))
  (bind (_hand _handskeletalcomponent) (Utilities|Struct|BreakOctoTentaclesStruct tentacle))
  ;[1 1 1] Attack Effect
  (for _array_element (Variables|Default|GetNS_TrailsArr)
    (if (Utilities|Enum|Equal(Enum) (.Hand (Utilities|Struct|BreakS_OctoHand _array_element)) _hand)
      (bind _returnvalue (AddComponent|AddNiagaraComponent true))
      (Class|NiagaraComponent|SetAutoDestroy _returnvalue true)
      (Transformation|AttachComponentToComponent _returnvalue _handskeletalcomponent "None" "KeepRelative" "KeepRelative" "KeepRelative" true))))

(event EventMovetoAttachPointEvent
  (params (tentacle :type Octo%20Tentacles%20Struct%20Structure))
  (bind (_hand _handskeletalcomponent) (Utilities|Struct|BreakOctoTentaclesStruct tentacle))
  ;[1 1 1] Trail Effect
  (for (_array_element _array_index) (Variables|Default|GetNS_TrailsArr)
    (if (Utilities|Enum|Equal(Enum) (.Hand (Utilities|Struct|BreakS_OctoHand _array_element)) _hand)
      (bind _returnvalue (AddComponent|AddNiagaraComponent true))
      (Transformation|AttachComponentToComponent _returnvalue _handskeletalcomponent "None" "KeepRelative" "KeepRelative" "KeepRelative" true)
      (Utilities|Array|SetArrayElem (Variables|Default|GetNS_TrailsArr) _array_index (Utilities|Struct|MakeS_OctoHand _hand _returnvalue)))))

(event EventAttachedEvent
  (params (tentacle :type Octo%20Tentacles%20Struct%20Structure))
  (bind _array (Utilities|Array|MakeArray 0.0 0.0 0.0 0.0))
  ;[1 1 1] Reset Values
  (Utilities|Struct|SetmembersinS_OctoHandAnim (Utilities|Array|Get(acopy) (Variables|Default|GetOctoHandAnimStruct) (.handIndex (Utilities|Struct|BreakOctoTentaclesStruct tentacle))) _array _array))

(event EventGrabbedEvent
  (params (tentacle :type Octo%20Tentacles%20Struct%20Structure))
  (bind _array (Utilities|Array|MakeArray 0.0 0.0 0.0 0.0))
  ;[1 0.7533 0.2102] If gragged object set zero hands section IK
  (Utilities|Struct|SetmembersinS_OctoHandAnim (Utilities|Array|Get(acopy) (Variables|Default|GetOctoHandAnimStruct) (.handIndex (Utilities|Struct|BreakOctoTentaclesStruct tentacle))) _array _array))

(fn ConstructionScript)
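; Boss monster variant of an octopus backpack component that finds targets ahead of its owner and deals fixed damage to actors passed to its damage event.
; A self-rescheduling timer runs a forward multi-object trace during battle mode, accepting pawns, physics-simulating components or "octo"-tagged hits.
; Hits update the target location and any existing marker; otherwise a visibility trace supplies the hit and the marker is destroyed.
; Marker spawning and widget creation are disconnected.
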(event Custom|TargetTraceObject
  (bind _returnvalue (Components|GetOwner))
  (bind _returnvalue_2 (Transformation|GetActorForwardVector _returnvalue))
  (bind _returnvalue_3 (Transformation|GetActorLocation _returnvalue))
  (bind _returnvalue_4 (* _returnvalue_2 5e+03))
  (bind _returnvalue_5 (+ _returnvalue_3 _returnvalue_4))
  ;[0.3834 1 0.1073] TargetTraceObject
  (Utilities|Time|SetTimerbyEvent (delegate Custom|TargetTraceObject) 0.1)
  (if (Variables|Default|GetbBattleMode)
    (Utilities|IsValid (Variables|Default|GetbackPackOcto)
      (:Is%20Valid
        (Variables|Default|SetbFoundTarget false)
        (bind _outhits (Class|KismetSystemLibrary|LineTraceMultiforObjects _returnvalue_3 _returnvalue_5 (Utilities|Array|MakeArray "ObjectTypeQuery4" "ObjectTypeQuery2" "ObjectTypeQuery3" "ObjectTypeQuery8") false (Variables|Default|GetIgnoreActors) "None" true))
        (bind _array_element (Utilities|Array|ForEachLoopwithBreak _outhits)
          (:LoopBody
            (if (.bBlockingHit (Collision|BreakHitResult _array_element))
              (if (Math|Boolean|ORBoolean (Physics|IsSimulatingPhysics (.HitComponent (Collision|BreakHitResult _array_element)) "None") (Components|ComponentHasTag (.HitComponent (Collision|BreakHitResult _array_element)) "octo") (Actor|ActorHasTag (.HitActor (Collision|BreakHitResult _array_element)) "octo") (.bSuccess (Utilities|Casting|CastToPawn (.HitActor (Collision|BreakHitResult _array_element)))))
                (Variables|Default|SetbFoundTarget true)
                (Utilities|IsValid (Variables|Default|GetBP_OctoTargetObject)
                  (:Is%20Valid
                    (Transformation|SetActorLocation (Variables|Default|GetBP_OctoTargetObject) (Transformation|GetActorLocation (.HitActor (Collision|BreakHitResult _array_element))) false false)
                    (Variables|Default|SetHitLocation _array_element)
                    (Variables|Default|SetbIsTargetLocation true))
                  (:Is%20Not%20Valid
                    (Variables|Default|SetHitLocation _array_element)
                    (Variables|Default|SetbIsTargetLocation true))))))
          (:Completed
            (if (not (Variables|Default|GetbFoundTarget))
              (bind _outhit (Collision|LineTraceByChannel _returnvalue_3 _returnvalue_5 "TraceTypeQuery1" false (Variables|Default|GetIgnoreActors) "None"))
              (Variables|Default|SetbIsTargetLocation false)
              (Variables|Default|SetHitLocation _outhit)
              (Utilities|IsValid (Variables|Default|GetBP_OctoTargetObject)
                (:Is%20Valid
                  (Actor|DestroyActor (Variables|Default|GetBP_OctoTargetObject))
                  (Variables|Default|SetBP_OctoTargetObject 0)))))))
      (:Is%20Not%20Valid
        (Variables|Default|SetbIsTargetLocation false :!label _label)))
    (else
      (goto _label))))

(event EventOctopusDamageActor
  (params (actor :type Actor%20Object%20Reference))
  ;[1 0.3082 0.01503] Apply Damage for Actors
  (Utilities|IsValid actor
    (:Is%20Valid
      (Game|Damage|ApplyDamage actor 5e+01 0 0))))

(event EventBeginPlay
  (Variables|Default|SetIgnoreActors (Utilities|Array|MakeArray (Components|GetOwner) (Variables|Default|GetbackPackOcto)))
  (CallFunction|TargetTraceObject))
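; Test boss actor that uses an octopus backpack component to grab and throw the player.
; On BeginPlay it registers the backpack and toggles battle mode, then Tick feeds InputScale, a horizontal direction away from the player, as movement.
; The Grab flag attacks, hides the player and spawns a physics robot mesh stand-in.
; The Throw flag throws it, then moves the player there and unhides them.
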(event Custom|SetInputScale
  (bind _returnvalue (Transformation|GetActorLocation))
  (bind _returnvalue_2 (Game|GetPlayerCharacter 0))
  (bind _returnvalue_3 (Transformation|GetActorLocation _returnvalue_2))
  (bind _returnvalue_4 (- _returnvalue _returnvalue_3))
  (bind _returnvalue_5 (Math|Vector|Normalize _returnvalue_4))
  (bind _output_get (Variables|Default|SetCurrentRotation (Transformation|GetActorRotation)))
  (if (> (- (.yaw _output_get) (.yaw (Variables|Default|GetPreRotation))) 0.0)
    ;[1 0.894 0] SET INPUT / X - LR, Y - FB , Z - UD
    (Variables|Default|SetInputScale (Math|Vector|MakeVector (.x _returnvalue_5) (.y _returnvalue_5) 0.0))
    (elif (== (- (.yaw _output_get) (.yaw (Variables|Default|GetPreRotation))) 0.0)
      ;[1 0.894 0] SET INPUT / X - LR, Y - FB , Z - UD
      (Variables|Default|SetInputScale (Math|Vector|MakeVector (.x _returnvalue_5) (.y _returnvalue_5) 0.0))
      (else
        ;[1 0.894 0] SET INPUT / X - LR, Y - FB , Z - UD
        (Variables|Default|SetInputScale (Math|Vector|MakeVector (.x _returnvalue_5) (.y _returnvalue_5) 0.0))))))

(event EventBeginPlay
  (bind _bp_octopusbackpackcomponent_my (Variables|Default|GetBP_OctopusBackpackComponent_My))
  ;[1 0.7451 0.06274] Register Octo Backpack
  (Class|OctopusBackpackComponent|RegisterOctopusBackpack _bp_octopusbackpackcomponent_my)
  (Class|OctopusBackpackComponent|OctopusBackpackBattleMode _bp_octopusbackpackcomponent_my (not (Variables|/Script/OctopusBackpack.OctopusBackpackComponent|GetbBattleMode _bp_octopusbackpackcomponent_my))))

(event EventTick
  (params (DeltaSeconds :type Float%20%28single-precision%29))
  (bind _returnvalue (Game|Player|GetPlayerPawn 0))
  (bind _bp_octopusbackpackcomponent_my (Variables|Default|GetBP_OctopusBackpackComponent_My))
  (bind _hitlocation (Variables|/Game/Monsters/BossMonster/Blueprints/BP_OctopusBackpackComponent_My.BP_OctopusBackpackComponent_My_C|GetHitLocation _bp_octopusbackpackcomponent_my))
  (Utilities|FlowControl|Sequence
    (:then_0
      (Class|OctopusBackpackComponent|SetMovementDirection (Variables|Default|GetBP_OctopusBackpackComponent_My) (Variables|Default|GetInputScale)))
    (:then_1
      (if (Variables|Default|GetbGrab)
        (Class|OctopusBackpackComponent|Attack _bp_octopusbackpackcomponent_my _hitlocation)
        (bind _returnvalue_2 (Game|SpawnActorfromClass "/Script/Engine.SkeletalMeshActor" (Math|Transform|MakeTransform (Transformation|GetActorLocation (Game|Player|GetPlayerPawn 0)) "0, 0, 0" "3.000000,3.000000,3.000000") "AlwaysSpawn" "MultiplyWithRoot" 0 0))
        (Components|SkeletalMesh|SetSkeletalMeshAsset (Variables|/Script/Engine.SkeletalMeshActor|GetSkeletalMeshComponent _returnvalue_2) "/Game/Asset/Character/Cute_Robot/Cute_Robot.Cute_Robot")
        (Physics|SetSimulatePhysics (Variables|/Script/Engine.SkeletalMeshActor|GetSkeletalMeshComponent _returnvalue_2) true)
        (Variables|/Script/Engine.ActorComponent|SetComponentTags (Variables|/Script/Engine.SkeletalMeshActor|GetSkeletalMeshComponent _returnvalue_2) (Variables|Default|GetComponent%20Tags))
        (Development|PrintString "GrabAttack 완료")
        (Variables|Default|SetbGrab false)
        (Rendering|SetActorHiddenInGame (Game|Player|GetPlayerPawn 0) true)
        (Variables|Default|SetIsPlayerAttacked true)))
    (:then_2
      (if (Variables|Default|GetbThrow)
        (Class|OctopusBackpackComponent|ThrowAll _bp_octopusbackpackcomponent_my _hitlocation 5e+01)
        (Development|PrintString "throw all")
        (Variables|Default|SetbThrow false)
        (Utilities|FlowControl|Delay 1.0)
        (Transformation|SetActorLocation _returnvalue (Transformation|GetActorLocation _returnvalue_2) false false)
        (Rendering|SetActorHiddenInGame _returnvalue false)
        (Actor|DestroyActor _returnvalue_2)
        (Variables|Default|SetIsPlayerAttacked false)))))

(fn ConstructionScript)
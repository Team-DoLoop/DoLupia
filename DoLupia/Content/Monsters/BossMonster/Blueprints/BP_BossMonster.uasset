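; Boss monster that uses an octopus backpack component for tentacle movement and a grab-and-throw attack on the player.
; Tick feeds InputScale, derived from the player-to-boss direction, into the backpack and polls Grab and Throw flags.
; Grab hides the player behind a physics-simulated hologram stand-in and blends to an external camera.
; Throw launches held targets or handles a missed grab, applies corresponding damage, and restores player and camera.
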(event Custom|SetInputScale
  (bind _returnvalue (Transformation|GetActorLocation))
  (bind _returnvalue_2 (Game|GetPlayerCharacter 0))
  (bind _returnvalue_3 (Transformation|GetActorLocation _returnvalue_2))
  (bind _returnvalue_4 (- _returnvalue _returnvalue_3))
  (bind _returnvalue_5 (Math|Vector|Normalize _returnvalue_4))
  (bind _output_get (Variables|Default|SetCurrentRotation (Transformation|GetActorRotation)))
  (if (> (- (.yaw _output_get) (.yaw (Variables|Default|GetPreRotation))) 0.0)
    ;[1 0.894 0] SET INPUT / X - LR, Y - FB , Z - UD
    (Variables|Default|SetInputScale (Math|Vector|MakeVector (.x _returnvalue_5) (.y _returnvalue_5) 0.0))
    (elif (== (- (.yaw _output_get) (.yaw (Variables|Default|GetPreRotation))) 0.0)
      ;[1 0.894 0] SET INPUT / X - LR, Y - FB , Z - UD
      (Variables|Default|SetInputScale (Math|Vector|MakeVector (.x _returnvalue_5) (.y _returnvalue_5) 0.0))
      (else
        ;[1 0.894 0] SET INPUT / X - LR, Y - FB , Z - UD
        (Variables|Default|SetInputScale (Math|Vector|MakeVector (.x _returnvalue_5) (.y _returnvalue_5) 0.0))))))

(event Custom|ResetBossLocation
  (Transformation|SetActorLocation "580.000000,680.000000,800.000000" false false))

(event EventBeginPlay
  (bind _bp_octopusbackpackcomponent_my (Variables|Default|GetBP_OctopusBackpackComponent_My))
  ;[1 0.7451 0.06274] Register Octo Backpack
  (Class|OctopusBackpackComponent|RegisterOctopusBackpack _bp_octopusbackpackcomponent_my)
  (Class|OctopusBackpackComponent|OctopusBackpackBattleMode _bp_octopusbackpackcomponent_my (not (Variables|/Script/OctopusBackpack.OctopusBackpackComponent|GetbBattleMode _bp_octopusbackpackcomponent_my)))
  (bind _returnvalue (Game|SpawnActorfromClass "/Script/Engine.TriggerBox" (Math|Conversions|ToTransform(Vector) (Transformation|GetActorLocation)) "Undefined" "MultiplyWithRoot" 0 0))
  (Variables|Default|SetCamTargetActor _returnvalue)
  (bind _asproject_dcharacter (Utilities|Casting|CastToProjectDCharacter (Game|Player|GetPlayerPawn 0)))
  (Variables|Default|SetPlayer _asproject_dcharacter))

(event EventTick
  (params (DeltaSeconds :type Float%20%28single-precision%29))
  (bind _bp_octopusbackpackcomponent_my (Variables|Default|GetBP_OctopusBackpackComponent_My))
  (bind _camtargetactor (Variables|Default|GetCamTargetActor))
  (bind _hitlocation (Variables|/Game/Monsters/BossMonster/Blueprints/BP_OctopusBackpackComponent_My.BP_OctopusBackpackComponent_My_C|GetHitLocation _bp_octopusbackpackcomponent_my))
  (Utilities|FlowControl|Sequence
    (:then_0
      (Class|OctopusBackpackComponent|SetMovementDirection (Variables|Default|GetBP_OctopusBackpackComponent_My) (Variables|Default|GetInputScale)))
    (:then_1
      (if (Variables|Default|GetbGrab)
        (Class|OctopusBackpackComponent|Attack _bp_octopusbackpackcomponent_my _hitlocation)
        (bind _returnvalue (Game|SpawnActorfromClass "/Script/Engine.SkeletalMeshActor" (Math|Transform|MakeTransform (Transformation|GetActorLocation (Game|Player|GetPlayerPawn 0)) "0, 0, 0" "4.000000,4.000000,4.000000") "AlwaysSpawn" "MultiplyWithRoot" 0 0))
        (Components|SkeletalMesh|SetSkeletalMeshAsset (Variables|/Script/Engine.SkeletalMeshActor|GetSkeletalMeshComponent _returnvalue) "/Game/Asset/Character/Cute_Robot/Cute_Robot.Cute_Robot")
        (Rendering|Material|SetMaterial (Variables|/Script/Engine.SkeletalMeshActor|GetSkeletalMeshComponent _returnvalue) 0 "/Game/Monsters/BossMonster/Blueprints/M_Hologram.M_Hologram")
        (Physics|SetSimulatePhysics (Variables|/Script/Engine.SkeletalMeshActor|GetSkeletalMeshComponent _returnvalue) true)
        (Variables|/Script/Engine.ActorComponent|SetComponentTags (Variables|/Script/Engine.SkeletalMeshActor|GetSkeletalMeshComponent _returnvalue) (Variables|Default|GetComponent%20Tags))
        (Variables|Default|SetPlayerTempMesh _returnvalue)
        (Variables|Default|SetbGrab false)
        (Variables|Default|SetIsDestroyed false)
        (Rendering|SetActorHiddenInGame (Game|Player|GetPlayerPawn 0) true)
        (Rendering|SetActorHiddenInGame (Class|GadgetComponent|GetSword (Class|ProjectDCharacter|GetGadgetComp (Variables|Default|GetPlayer))) true)
        (Class|ProjectDCharacter|PlayerGrabEnd (Variables|Default|GetPlayer))
        (Utilities|FlowControl|Delay 1.0)
        (bind _playertempmesh (Variables|Default|GetPlayerTempMesh)
          (:then
            ;[1 1 1] 외부 카메라
            (Transformation|SetActorLocationAndRotation _camtargetactor (+ (Transformation|GetActorLocation _playertempmesh) "-303.321374,-203.922338,330.302803") "-46.000000,33.000000,0.000000")
            (Game|Player|SetViewTargetwithBlend (Game|GetPlayerController 0) _camtargetactor 0.5 "VTBlend_Cubic" 0.0 false)
            (Components|Animation|PlayAnimation (Variables|/Script/Engine.SkeletalMeshActor|GetSkeletalMeshComponent _returnvalue) "/Game/Monsters/BossMonster/Animation/Laying_Seizure_Anim_mixamo_com1.Laying_Seizure_Anim_mixamo_com1" true))
          (:else))))
    (:then_3
      (if (Variables|Default|GetbThrow)
        (bind _asbp_octopus_backpack_actor_my (Utilities|Casting|CastToBP_OctopusBackpackActor_My (Variables|/Script/Engine.ChildActorComponent|GetChildActor (Variables|Default|GetChildActor))))
        (if (Variables|/Game/Monsters/BossMonster/Blueprints/BP_OctopusBackpackActor_My.BP_OctopusBackpackActor_My_C|GetGrabTarget _asbp_octopus_backpack_actor_my)
          (Class|OctopusBackpackComponent|ThrowAll (Variables|Default|GetBP_OctopusBackpackComponent_My) _hitlocation 5.0)
          (Rendering|SetActorHiddenInGame _returnvalue true)
          ;[1 0.08044 0.1501] 공격 판정
          (bind _asbp_player (Utilities|Casting|CastToBP_Player (Game|Player|GetPlayerPawn 0)))
          (Class|ProjectDCharacter|TakeHit _asbp_player "BASIC" "NONE" 5e+01)
          (Variables|Default|SetbThrow false)
          (Game|Player|SetViewTargetwithBlend (Game|GetPlayerController 0) (Variables|Default|GetPlayerTempMesh) 1.0 "VTBlend_Cubic" 0.0 false)
          (Utilities|FlowControl|Delay 1.5)
          (Transformation|SetActorLocation (Game|Player|GetPlayerPawn 0) (+ (Transformation|GetActorLocation _returnvalue) "0.000000,0.000000,10.000000") false false)
          ;[1 0.8949 0.8849] 이 구간에서 카메라 원래 시점으로 복귀 필요!!!!!!!!
          (Actor|DestroyActor _returnvalue)
          (Rendering|SetActorHiddenInGame (Game|GetPlayerCharacter 0) false)
          (Rendering|SetActorHiddenInGame (Class|GadgetComponent|GetSword (Class|ProjectDCharacter|GetGadgetComp (Variables|Default|GetPlayer))) false)
          (Game|Player|SetViewTargetwithBlend (Game|GetPlayerController 0) (Variables|Default|GetPlayer) 1.0 "VTBlend_EaseOut" 0.0 false)
          (Animation|Montage|PlayMontage (Variables|/Script/Engine.Character|GetMesh (Variables|Default|GetPlayer)) "/Game/Player/Animation/Hit/M_PlayerGrabEnd.M_PlayerGrabEnd"
            (:OnCompleted
              (Variables|Default|SetIsDestroyed true)))
          (else
            ;[0.1645 0.5005 1] 안잡혔을 떄, 카메라 원래 시점으로 복귀하고 메시 삭제
            ;;[1 0.08044 0.1501] 공격 판정
            (bind _asbp_player_2 (Utilities|Casting|CastToBP_Player (Game|Player|GetPlayerPawn 0)))
            (Class|ProjectDCharacter|TakeHit _asbp_player_2 "BASIC" "NONE" 2e+01)
            (Variables|Default|SetbThrow false)
            (Game|Player|SetViewTargetwithBlend (Game|GetPlayerController 0) (Variables|Default|GetPlayer) 0.7 "VTBlend_Cubic" 0.0 false)
            (if (not (Variables|Default|GetIsDestroyed))
              (Actor|DestroyActor _returnvalue)
              (Variables|Default|SetIsDestroyed true)
              (Rendering|SetActorHiddenInGame (Game|Player|GetPlayerPawn 0) false)
              (Rendering|SetActorHiddenInGame (Class|GadgetComponent|GetSword (Class|ProjectDCharacter|GetGadgetComp (Variables|Default|GetPlayer))) false)
              (Animation|Montage|PlayMontage (Variables|/Script/Engine.Character|GetMesh (Variables|Default|GetPlayer)) "/Game/Player/Animation/Hit/M_PlayerGrabEnd.M_PlayerGrabEnd" 0.0 1.0))))))))

(event Input|KeyboardEvents|L
  (params (Key :type Key%20Structure :default "None")))

(fn ConstructionScript)
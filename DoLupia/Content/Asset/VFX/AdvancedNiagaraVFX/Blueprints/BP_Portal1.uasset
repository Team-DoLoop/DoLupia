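; Portal actor that tracks a BP_Walk character passing through its Box trigger and publishes plane-relative values to a material parameter collection.
; On overlap it caches the character's SkeletalMesh and attaches the NS_AttackVFXMove Niagara effect to it.
; Each Tick it writes MPC_Angle's Amount from the mesh's scaled, negated world-Y offset from the portal actor, and Angle from the Plane's up vector.
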(event OnComponentBeginOverlap(Box)
  (params (OverlappedComponent :type Primitive%20Component%20Object%20Reference) (OtherActor :type Actor%20Object%20Reference) (OtherComp :type Primitive%20Component%20Object%20Reference) (OtherBodyIndex :type Integer) (bFromSweep :type Boolean) (SweepResult :type Hit%20Result%20Structure%20%28by%20ref%29))
  (bind _asbp_walk (Utilities|Casting|CastToBP_Walk OtherActor))
  (Variables|Default|SetSkeletal%20Mesh (Variables|/Game/Asset/VFX/AdvancedNiagaraVFX/Blueprints/BP_Walk.BP_Walk_C|GetSkeletalMesh _asbp_walk))
  (Niagara|SpawnSystemAttached "/Game/Asset/VFX/AdvancedNiagaraVFX/Particles/DashTrail/NS_AttackVFXMove.NS_AttackVFXMove" (Variables|Default|GetSkeletal%20Mesh) "None" "0, 0, 0" "0, 0, 0" "KeepRelativeOffset" false))

(event EventTick
  (params (DeltaSeconds :type Float%20%28single-precision%29))
  (Variables|Default|GetSkeletal%20Mesh
    (:then
      (Rendering|Material|SetScalarParameterValue "/Game/Asset/VFX/AdvancedNiagaraVFX/Materials/MPC/MPC_Angle.MPC_Angle" "Amount" (* (/ (- (.y (Transformation|GetWorldLocation (Variables|Default|GetSkeletal%20Mesh))) (.y (.location (Transformation|GetActorTransform (Components|GetOwner (Variables|Default|GetPlane)))))) 1e+01) -1.0) :!class /Script/Engine.KismetMaterialLibrary)
      (Rendering|Material|SetVectorParameterValue "/Game/Asset/VFX/AdvancedNiagaraVFX/Materials/MPC/MPC_Angle.MPC_Angle" "Angle" (Math|Conversions|ToLinearColor(Vector) (Math|Vector|GetUpVector (Variables|Default|GetPlane))) :!class /Script/Engine.KismetMaterialLibrary))
    (:else)))

(fn ConstructionScript)
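; Quest actor that routes keyboard input to the 2048 minigame in the level.
; On BeginPlay it casts the player controller to BP_TopDownPlayerController and enables input on itself.
; Each arrow key finds BP_MiniGame2048 via GetActorOfClass, squashes the grid in that direction, spawns a new number and redraws.
; Enter calls GameClear and clears the grid widgets.
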(event EventBeginPlay
  (bind _asbp_top_down_player_controller (Utilities|Casting|CastToBP_TopDownPlayerController (Game|GetPlayerController 0)))
  (bind _output_get (Variables|Default|Setcontroller _asbp_top_down_player_controller))
  (Input|EnableInput _output_get))

(event Collision|EventActorBeginOverlap
  (params (OtherActor :type Actor%20Object%20Reference)))

(event EventTick
  (params (DeltaSeconds :type Float%20%28single-precision%29)))

(event Input|KeyboardEvents|Up
  (params (Key :type Key%20Structure :default "None"))
  (:Pressed
    (bind _returnvalue (Actor|GetActorOfClass "/Game/UserInterface/MiniGame/BP_MiniGame2048.BP_MiniGame2048_C"))
    (Class|Grid2048|Squash _returnvalue 2)
    (Class|Grid2048|NewNumber _returnvalue)
    (Class|Grid2048|Draw _returnvalue)))

(event Input|KeyboardEvents|Down
  (params (Key :type Key%20Structure :default "None"))
  (:Pressed
    (bind _returnvalue (Actor|GetActorOfClass "/Game/UserInterface/MiniGame/BP_MiniGame2048.BP_MiniGame2048_C"))
    (Class|Grid2048|Squash _returnvalue 3)
    (Class|Grid2048|NewNumber _returnvalue)
    (Class|Grid2048|Draw _returnvalue)))

(event Input|KeyboardEvents|Right
  (params (Key :type Key%20Structure :default "None"))
  (:Pressed
    (bind _returnvalue (Actor|GetActorOfClass "/Game/UserInterface/MiniGame/BP_MiniGame2048.BP_MiniGame2048_C"))
    (Class|Grid2048|Squash _returnvalue 1)
    (Class|Grid2048|NewNumber _returnvalue)
    (Class|Grid2048|Draw _returnvalue)))

(event Input|KeyboardEvents|Left
  (params (Key :type Key%20Structure :default "None"))
  (:Pressed
    (bind _returnvalue (Actor|GetActorOfClass "/Game/UserInterface/MiniGame/BP_MiniGame2048.BP_MiniGame2048_C"))
    (Class|Grid2048|Squash _returnvalue)
    (Class|Grid2048|NewNumber _returnvalue)
    (Class|Grid2048|Draw _returnvalue)))

(event Input|KeyboardEvents|Enter
  (params (Key :type Key%20Structure :default "None"))
  (:Pressed
    (bind _returnvalue (Actor|GetActorOfClass "/Game/UserInterface/MiniGame/BP_MiniGame2048.BP_MiniGame2048_C"))
    (Class|Grid2048|GameClear _returnvalue)
    (Class|Grid2048|ClearGridWidgets _returnvalue)))

(fn ConstructionScript)
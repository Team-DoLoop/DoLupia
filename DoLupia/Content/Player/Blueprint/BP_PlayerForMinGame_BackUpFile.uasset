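; Player Blueprint, named as a backup file, that drives the 2048 minigame from keyboard input.
; BeginPlay creates the WBP_2048Main widget and adds it to the viewport.
; Each arrow key finds the BP_MiniGame2048 actor, calls Squash with a direction index, then calls NewNumber and Draw, without checking whether the move changed the board.
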(event EventBeginPlay
  (bind _returnvalue (UserInterface|CreateWidget "/Game/UserInterface/MiniGame/WBP_2048Main.WBP_2048Main_C"))
  (UserInterface|Viewport|AddtoViewport _returnvalue 0))

(event Input|KeyboardEvents|Up
  (params (Key :type Key%20Structure))
  (:Pressed
    (bind _returnvalue (Actor|GetActorOfClass "/Game/UserInterface/MiniGame/BP_MiniGame2048.BP_MiniGame2048_C"))
    (Class|Grid2048|Squash _returnvalue 2)
    (Class|Grid2048|NewNumber _returnvalue)
    (Class|Grid2048|Draw _returnvalue)))

(event Input|KeyboardEvents|Down
  (params (Key :type Key%20Structure))
  (:Pressed
    (bind _returnvalue (Actor|GetActorOfClass "/Game/UserInterface/MiniGame/BP_MiniGame2048.BP_MiniGame2048_C"))
    (Class|Grid2048|Squash _returnvalue 3)
    (Class|Grid2048|NewNumber _returnvalue)
    (Class|Grid2048|Draw _returnvalue)))

(event Input|KeyboardEvents|Right
  (params (Key :type Key%20Structure))
  (:Pressed
    (bind _returnvalue (Actor|GetActorOfClass "/Game/UserInterface/MiniGame/BP_MiniGame2048.BP_MiniGame2048_C"))
    (Class|Grid2048|Squash _returnvalue 1)
    (Class|Grid2048|NewNumber _returnvalue)
    (Class|Grid2048|Draw _returnvalue)))

(event Input|KeyboardEvents|Left
  (params (Key :type Key%20Structure))
  (:Pressed
    (bind _returnvalue (Actor|GetActorOfClass "/Game/UserInterface/MiniGame/BP_MiniGame2048.BP_MiniGame2048_C"))
    (Class|Grid2048|Squash _returnvalue)
    (Class|Grid2048|NewNumber _returnvalue)
    (Class|Grid2048|Draw _returnvalue)))

(fn ConstructionScript)
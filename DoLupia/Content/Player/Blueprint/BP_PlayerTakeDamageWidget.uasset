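; BP_PlayerTakeDamageWidget is a floating damage-text actor in the player folder, built on a text render component rather than UMG.
; On BeginPlay it caches its location and the text's world size, then plays a timeline.
; The timeline offsets the text vertically from the start position and scales its size, and the actor destroys itself when it finishes.
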(event EventBeginPlay
  (bind _damagetextrender (Variables|Default|GetDamageTextRender))
  (Variables|Default|SetStartPos (Transformation|GetActorLocation))
  (Variables|Default|SetStartSize (Variables|/Script/Engine.TextRenderComponent|GetWorldSize (Variables|Default|GetDamageTextRender)))
  (bind (_direction _newtrack_0 _newtrack_1) (Timeline|TakeDamageTextTimeline Play)
    (:Update
      (Transformation|SetWorldLocation _damagetextrender (+ (Variables|Default|GetStartPos) (Math|Vector|MakeVector 0.0 0.0 (.Z (Math|Vector|BreakVector _newtrack_0)))) false false)
      (Rendering|Components|TextRender|SetWorldSize _damagetextrender (* (Variables|Default|GetStartSize) _newtrack_1)))
    (:Finished
      (Actor|DestroyActor))))

(event Collision|EventActorBeginOverlap
  (params (OtherActor :type Actor%20Object%20Reference)))

(event EventTick
  (params (DeltaSeconds :type Float%20%28single-precision%29)))

(fn ConstructionScript)